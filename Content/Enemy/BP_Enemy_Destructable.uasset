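; Destructible enemy that turns to face the hero and fires projectiles on a looping timer once alerted by capsule overlap or being hit.
; Mesh hits play sound, subtract health and flash emission; at zero health it explodes and is destroyed.
; Separate events clear the fire timer, reset its DoOnce gate and clear alert flags.
; BeginPlay caches the hero and randomizes a vertical bob, but that timeline logic is unwired.
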(event OnComponentHit(EnemyMesh)
  (params (HitComponent :type Primitive%20Component%20Object%20Reference) (OtherActor :type Actor%20Object%20Reference) (OtherComp :type Primitive%20Component%20Object%20Reference) (NormalImpulse :type Vector :default "0, 0, 0") (Hit :type Hit%20Result%20Structure%20%28by%20ref%29))
  (bind _location (Collision|BreakHitResult Hit))
  (Development|PrintString "Hello")
  ;[1 1 1] Call hit from some actor / Enemy Damage / Destroy actor
  ;;[1 0.3961 0] Play Sound Hit
  (Audio|SpawnSoundatLocation "/Game/Audio/SoundEffects/Enemy_Hit1.Enemy_Hit1" _location "0, 0, 0" 1.0 1.0 0.0 0 0)
  (Variables|Default|SetIsHeroHere true)
  (Variables|Default|SetEnemyHealth (- (Variables|Default|GetEnemyHealth) (Variables|Default|GetDamageTaken)))
  (if (<= (Variables|Default|GetEnemyHealth) 0.0)
    (CallFunction|EventDead)
    ;;[1 0.3961 0] Play Sound Hit
    (Audio|SpawnSoundatLocation "/Game/Audio/SoundEffects/Enemy_Dead1.Enemy_Dead1" _location "0, 0, 0" 1.0 1.0 0.0 0 0)
    (Effects|SpawnEmitteratLocation "/Game/StarterContent/Particles/P_Explosion.P_Explosion" _location)
    (Physics|SetSimulatePhysics (Variables|Default|GetEnemyMesh) false)
    (Actor|DestroyActor)
    (else
      (Rendering|Material|SetScalarParameterValueonMaterials (Variables|Default|GetEnemyMesh) "Emission" 1.0)
      (Utilities|FlowControl|Delay 0.1)
      (Rendering|Material|SetScalarParameterValueonMaterials (Variables|Default|GetEnemyMesh) "Emission" 6e+01))))

(event OnComponentBeginOverlap(Capsule)
  (params (OverlappedComponent :type Primitive%20Component%20Object%20Reference) (OtherActor :type Actor%20Object%20Reference) (OtherComp :type Primitive%20Component%20Object%20Reference) (OtherBodyIndex :type Integer) (bFromSweep :type Boolean) (SweepResult :type Hit%20Result%20Structure%20%28by%20ref%29))
  ;[1 1 1] Activate AI perception on sight
  (Variables|Default|SetIsHeroOnSight true))

(event OnComponentEndOverlap(Capsule)
  (params (OverlappedComponent :type Primitive%20Component%20Object%20Reference) (OtherActor :type Actor%20Object%20Reference) (OtherComp :type Primitive%20Component%20Object%20Reference) (OtherBodyIndex :type Integer))
  ;[1 1 1] Deactivate AI perception on sight
)

(event Custom|EventDead)

(event Custom|StopEnemy
  ;[1 1 1] Stop Enemy
  (Utilities|Time|ClearTimerbyFunctionName 0 "Fire"))

(event Custom|RestartEnemyFire
  ;[1 1 1] Set AI perception to sight HeroChar / Fire
  (Utilities|FlowControl|DoOnce false) ; enters at Reset
)

(event Custom|RestartEnemy
  ;[1 1 1] Restart Enemy
  (Variables|Default|SetIsHeroOnSight false)
  (Variables|Default|SetIsHeroHere false))

(event EventBeginPlay
  (bind _returnvalue (Transformation|GetActorLocation))
  (Utilities|FlowControl|Sequence
    (:then_0
      ;[1 1 1] Get actor location and set start and location from self / Set timeline play rate
      (Variables|Default|SetStartLocation _returnvalue)
      (Variables|Default|SetEndLocation (+ _returnvalue (Math|Vector|MakeVector 0.0 0.0 (Math|Random|RandomFloatinRange 5e+01 1e+02))))
      (Components|Timeline|SetPlayRate (Variables|Default|GetEnemyLoopDestructable) (Math|Random|RandomFloatinRange 1.0 2.0)))
    (:then_1
      ;[1 1 1] Get HeroChar refer
      (bind _asbp_hero_char (Utilities|Casting|CastToBP_HeroChar (Game|GetPlayerCharacter 0)))
      (Variables|Default|SetHeroCharRefer _asbp_hero_char))))

(event EventTick
  (params (DeltaSeconds :type Float%20%28single-precision%29))
  ;[1 1 1] Set AI perception to sight HeroChar / Fire
  (if (or (Variables|Default|GetIsHeroHere) (Variables|Default|GetIsHeroOnSight))
    (Utilities|FlowControl|Sequence
      (:then_0
        (Transformation|SetActorRotation (Math|Rotator|FindLookatRotation (Transformation|GetActorLocation) (Transformation|GetActorLocation (Variables|Default|GetHeroCharRefer)))))
      (:then_1
        (Utilities|FlowControl|DoOnce false
          (:Completed
            (Utilities|Time|SetTimerbyFunctionName 0 "Fire" (/ 1.0 (Variables|Default|GetShootPerSecond)) true)))))))

(fn ConstructionScript)

(fn Fire
  (bind _arrowprojectil (Variables|Default|GetArrowProjectil))
  (Game|SpawnActorfromClass "/Game/Enemy/BP_ProjectilEnemy.BP_ProjectilEnemy_C" (Transformation|GetWorldTransform _arrowprojectil) "Undefined" 0 0)
  ;[1 0.3961 0] Play Sound Fire
  (Audio|SpawnSoundatLocation "/Game/Audio/SoundEffects/Enemy_Fire1.Enemy_Fire1" (Transformation|GetWorldLocation _arrowprojectil) "0, 0, 0" 1.0 1.0 0.0 0 0))