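; BP_Enemy_Boss is a boss enemy that counts toward the game's win condition when it dies.
; On BeginPlay it runs the parent logic and caches the gameplay game mode.
; Its death event increments the game mode's dead-boss counter and calls CheckWinGame; all other behavior is left to the parent class.
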(event EventBeginPlay
  (|CallParentFunction)
  (bind _asbp_gameplay_game_mode (Utilities|Casting|CastToBP_GameplayGameMode (Game|GetGameMode)))
  (Variables|Default|SetBP_GameModeRefer _asbp_gameplay_game_mode))

(event Collision|EventActorBeginOverlap
  (params (OtherActor :type Actor%20Object%20Reference)))

(event EventTick
  (params (DeltaSeconds :type Float%20%28single-precision%29))
  (|CallParentFunction DeltaSeconds) ; This node is disabled and will not be called.\nDrag off pins to build functionality.
)

(event EventEventDead
  (bind _bp_gamemoderefer (Variables|Default|GetBP_GameModeRefer))
  (Variables|/Game/GameLogic/BP_GameplayGameMode.BP_GameplayGameMode_C|SetNumberOfDeadEnemyBosses _bp_gamemoderefer (+ (Variables|/Game/GameLogic/BP_GameplayGameMode.BP_GameplayGameMode_C|GetNumberOfDeadEnemyBosses _bp_gamemoderefer) 1))
  (Default|CheckWinGame (Variables|Default|GetBP_GameModeRefer)))

(fn ConstructionScript
  (|CallParentFunction))