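; BP_ProjectilEnemy is an enemy projectile actor that damages the hero character on impact.
; On BeginPlay it caches the player as BP_HeroChar and gives itself a short lifespan.
; On hit it calls HeroDamage with its Damage value if it struck the cached hero, then destroys itself after a brief delay whatever it hit.
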(event Collision|EventHit
  (params (MyComp :type Primitive%20Component%20Object%20Reference) (Other :type Actor%20Object%20Reference) (OtherComp :type Primitive%20Component%20Object%20Reference) (bSelfMoved :type Boolean) (HitLocation :type Vector :default "0, 0, 0") (HitNormal :type Vector :default "0, 0, 0") (NormalImpulse :type Vector :default "0, 0, 0") (Hit :type Hit%20Result%20Structure%20%28by%20ref%29))
  ;[1 1 1] Destroy projectil actor
  (if (== Other (Variables|Default|GetBP_HeroCharRefer))
    (Default|HeroDamage (Variables|Default|GetBP_HeroCharRefer) (Variables|Default|GetDamage))
    (Utilities|FlowControl|Delay 0.1)
    (Actor|DestroyActor)
    (else
      (Utilities|FlowControl|Delay 0.1)
      (Actor|DestroyActor))))

(event EventBeginPlay
  ;[1 1 1] Cast hero char blueprint
  (bind _asbp_hero_char (Utilities|Casting|CastToBP_HeroChar (Game|GetPlayerCharacter 0)))
  (Variables|Default|SetBP_HeroCharRefer _asbp_hero_char)
  (Actor|SetLifeSpan 2.0))

(fn ConstructionScript)