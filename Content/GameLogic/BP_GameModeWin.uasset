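; BP_GameModeWin is the Blueprint that, judging by its name, serves as the game mode for the win state, staging the ending and credits.
; On BeginPlay it blends the first player's view to the first CameraActor found, then calls WinGame on every BP_Totem.
; Inside that totem loop it also adds a CreditsMenu widget, enables input and shows the mouse cursor, so each totem spawns its own menu.
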(event EventBeginPlay
  (bind _returnvalue (Game|GetPlayerController 0))
  (bind _outactors (Actor|GetAllActorsOfClass "/Script/Engine.CameraActor"))
  (Game|Player|SetViewTargetwithBlend (Game|GetPlayerController 0) (Utilities|Array|Get(acopy) _outactors) 0.0 "VTBlend_Linear" 0.0 false)
  (bind _outactors_2 (Actor|GetAllActorsOfClass "/Game/Objects/Totem/BP_Totem.BP_Totem_C"))
  (for _array_element _outactors_2
    (Default|WinGame _array_element)
    (bind _returnvalue_2 (UserInterface|CreateWidget "/Game/HUD/CreditsMenu.CreditsMenu_C"))
    (UserInterface|Viewport|AddtoViewport _returnvalue_2 0)
    (Input|EnableInput _returnvalue)
    (Variables|/Script/Engine.PlayerController|SetbShowMouseCursor _returnvalue true)))

(fn ConstructionScript)