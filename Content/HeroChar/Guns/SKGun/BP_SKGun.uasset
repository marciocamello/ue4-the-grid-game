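; BP_SKGun is a gun for BP_HeroChar that shoots projectiles, caching the player character on BeginPlay.
; Fire plays the gun sound and spawns BP_ProjectilBase at the hero's ArrowProjectil transform.
; ActiveTrigger fires at once and sets a looping timer paced by ShooterPerSecond, though that timer call names no function.
; DeactiveTrigger clears the timer named "Fire".
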(event Custom|DeactiveTrigger
  ;[1 1 1] Active Trigger / Deactive Trigger
  (Utilities|Time|ClearTimerbyFunctionName 0 "Fire"))

(event Custom|ActiveTrigger
  ;[1 1 1] Active Trigger / Deactive Trigger
  (CallFunction|Fire)
  (Utilities|Time|SetTimerbyFunctionName 0 "" (/ 1.0 (Variables|Default|GetShooterPerSecond)) true))

(event EventBeginPlay
  ;[1 1 1] Get HeroChar reference
  (bind _asbp_hero_char (Utilities|Casting|CastToBP_HeroChar (Game|GetPlayerCharacter 0)))
  (Variables|Default|SetHeroRefer _asbp_hero_char))

(fn ConstructionScript)

(fn Fire
  (bind _herorefer (Variables|Default|GetHeroRefer))
  (bind _arrowprojectil (Variables|/Game/HeroChar/BP_HeroChar.BP_HeroChar_C|GetArrowProjectil _herorefer))
  (bind _returnvalue (Transformation|GetWorldTransform _arrowprojectil))
  ;[1 1 1] Play Sound Fire
  (Audio|PlaySoundatLocation "/Game/Audio/SoundEffects/SK_Gun2_Cue.SK_Gun2_Cue" (.location _returnvalue) "0, 0, 0" 1.0 1.0 0.0 0 0 0)
  (Game|SpawnActorfromClass "/Game/HeroChar/Guns/BP_ProjectilBase.BP_ProjectilBase_C" (Math|Transform|MakeTransform (.location _returnvalue) (.rotation _returnvalue) (.scale _returnvalue)) "Undefined" 0 0))