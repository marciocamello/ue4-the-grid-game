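; BP_ProjectilBase is a projectile base for hero guns that carries a damage value readable through GetProjectileDamage.
; On BeginPlay it sets a short lifespan and creates a dynamic material instance on its mesh from the projectile material.
; On hitting a valid actor it spawns the weapon hit effect at the mesh transform, then after a brief delay destroys both the effect and itself.
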(event Collision|EventHit
  (params (MyComp :type Primitive%20Component%20Object%20Reference) (Other :type Actor%20Object%20Reference) (OtherComp :type Primitive%20Component%20Object%20Reference) (bSelfMoved :type Boolean) (HitLocation :type Vector :default "0, 0, 0") (HitNormal :type Vector :default "0, 0, 0") (NormalImpulse :type Vector :default "0, 0, 0") (Hit :type Hit%20Result%20Structure%20%28by%20ref%29))
  ;[1 1 1] Projectil add sparks particle and destroy
  (Utilities|IsValid Other
    (:Is%20Valid
      (bind _returnvalue (Game|SpawnActorfromClass (Variables|Default|GetWeaponHitFX) (Transformation|GetWorldTransform (Variables|Default|GetProjectilMesh)) "Undefined" 0 0))
      (Utilities|IsValid _returnvalue
        (:Is%20Valid
          (Utilities|FlowControl|Delay 0.1)
          (Actor|DestroyActor _returnvalue)
          (Actor|DestroyActor))))))

(event EventBeginPlay
  (Actor|SetLifeSpan 2.0)
  (Rendering|Material|CreateDynamicMaterialInstance (Variables|Default|GetProjectilMesh) 0 (Variables|Default|GetProjectileMaterial) "None" :!class /Script/Engine.PrimitiveComponent))

(fn ConstructionScript)

(fn GetProjectileDamage
  (return (Variables|Default|GetDamage)))