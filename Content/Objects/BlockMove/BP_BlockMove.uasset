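; BP_BlockMove is a block actor with a glowing material and a timeline meant to slide it between two positions.
; BeginPlay sets the BlockMove timeline's play rate and gives the Block a dynamic M_Glow material tinted by BaseColor.
; The timeline's update lerps the Block's relative location from StartLocation to EndLocation.
; No graph input starts the timeline, so movement depends on it being started elsewhere, such as by autoplay.
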(event EventBeginPlay
  (Components|Timeline|SetPlayRate (Variables|Default|GetBlockMove) (Variables|Default|GetTimelineRate))
  (bind _returnvalue (Rendering|Material|CreateDynamicMaterialInstance (Variables|Default|GetBlock) 1 "/Game/Materials/M_Glow.M_Glow" "None" :!class /Script/Engine.PrimitiveComponent))
  (Rendering|Material|SetVectorParameterValue _returnvalue "BaseColor" (Variables|Default|GetBaseColor) :!class /Script/Engine.MaterialInstanceDynamic))

(event Collision|EventActorBeginOverlap
  (params (OtherActor :type Actor%20Object%20Reference)))

(event EventTick
  (params (DeltaSeconds :type Float%20%28single-precision%29)))

(fn ConstructionScript)