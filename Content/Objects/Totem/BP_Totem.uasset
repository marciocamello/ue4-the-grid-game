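; Totem actor that activates when interacted with, provided the game mode reports the matching pink, blue or green key as picked.
; InteractTotem switches on key type through a DoOnce, which precedes the key check.
; Activation plays the rim timeline, brightens the glow, spawns a color-tinted BP_KeyFixed, then has the game mode count and check active totems.
; WinGame shows the rim and boosts emission on the construction-script dynamic material.
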(event Custom|ActivatePinkKey
  (bind _totemcolor (CallFunction|GetTotemColor "NewEnumerator0"))
  (bind _bp_gamemoderefer (Variables|Default|GetBP_GameModeRefer))
  ;[1 1 1] Activate Pink Key
  (if (Variables|/Game/GameLogic/BP_GameplayGameMode.BP_GameplayGameMode_C|GetisPickPinkKey (Variables|Default|GetBP_GameModeRefer))
    (CallFunction|PlayTotemAnimationandSetEmission)
    (bind _returnvalue (CallFunction|SpawnKey))
    (CallFunction|ChangeActiveKeyColor (Variables|/Game/Objects/Key/BP_KeyFixed.BP_KeyFixed_C|GetFrame1 _returnvalue) _totemcolor 5e+01)
    (CallFunction|ChangeActiveKeyColor (Variables|/Game/Objects/Key/BP_KeyFixed.BP_KeyFixed_C|GetFrame2 _returnvalue) _totemcolor 5e+01)
    (Default|IncrementNumberTotemsActive _bp_gamemoderefer)
    (Default|CheckAllTotemsActive _bp_gamemoderefer)))

(event Custom|ActivateBlueKey
  (bind _totemcolor (CallFunction|GetTotemColor "NewEnumerator1"))
  (bind _bp_gamemoderefer (Variables|Default|GetBP_GameModeRefer))
  ;[1 1 1] Activate Blue Key
  (if (Variables|/Game/GameLogic/BP_GameplayGameMode.BP_GameplayGameMode_C|GetisPickBlueKey (Variables|Default|GetBP_GameModeRefer))
    (CallFunction|PlayTotemAnimationandSetEmission)
    (bind _returnvalue (CallFunction|SpawnKey))
    (CallFunction|ChangeActiveKeyColor (Variables|/Game/Objects/Key/BP_KeyFixed.BP_KeyFixed_C|GetFrame1 _returnvalue) _totemcolor 5e+01)
    (CallFunction|ChangeActiveKeyColor (Variables|/Game/Objects/Key/BP_KeyFixed.BP_KeyFixed_C|GetFrame2 _returnvalue) _totemcolor 5e+01)
    (Default|IncrementNumberTotemsActive _bp_gamemoderefer)
    (Default|CheckAllTotemsActive _bp_gamemoderefer)))

(event Custom|ActivateGreenKey
  (bind _totemcolor (CallFunction|GetTotemColor "NewEnumerator2"))
  (bind _bp_gamemoderefer (Variables|Default|GetBP_GameModeRefer))
  ;[1 1 1] Activate Green Key
  (if (Variables|/Game/GameLogic/BP_GameplayGameMode.BP_GameplayGameMode_C|GetisPickGreenKey (Variables|Default|GetBP_GameModeRefer))
    (CallFunction|PlayTotemAnimationandSetEmission)
    (bind _returnvalue (CallFunction|SpawnKey))
    (CallFunction|ChangeActiveKeyColor (Variables|/Game/Objects/Key/BP_KeyFixed.BP_KeyFixed_C|GetFrame1 _returnvalue) _totemcolor 5e+01)
    (CallFunction|ChangeActiveKeyColor (Variables|/Game/Objects/Key/BP_KeyFixed.BP_KeyFixed_C|GetFrame2 _returnvalue) _totemcolor 5e+01)
    (Default|IncrementNumberTotemsActive _bp_gamemoderefer)
    (Default|CheckAllTotemsActive _bp_gamemoderefer)))

(event Custom|WinGame
  (bind _totemmaterial (Variables|Default|GetTotemMaterial))
  ;[1 1 1] Win Game
  (Components|Timeline|PlayfromStart (Variables|Default|GetTotemRimTimeline))
  (Rendering|SetVisibility (Variables|Default|GetTotemRim) true false)
  (Rendering|Material|SetScalarParameterValue _totemmaterial "Emission" 1e+02 :!class /Script/Engine.MaterialInstanceDynamic)
  (Rendering|Material|SetVectorParameterValue _totemmaterial "BaseColor" (Variables|Default|GetBaseColor) :!class /Script/Engine.MaterialInstanceDynamic))

(event EventBeginPlay
  ;[1 1 1] Cast Game Mode
  (bind _asbp_gameplay_game_mode (Utilities|Casting|CastToBP_GameplayGameMode (Game|GetGameMode)))
  (Variables|Default|SetBP_GameModeRefer _asbp_gameplay_game_mode))

(event EventInteractTotem
  (switch Utilities|FlowControl|Switch|SwitchonEKeys (Variables|Default|GetTotemKeyType)
    (:NewEnumerator0
      (Utilities|FlowControl|DoOnce false
        (:Completed
          (CallFunction|ActivatePinkKey))))
    (:NewEnumerator1
      (Utilities|FlowControl|DoOnce false
        (:Completed
          (CallFunction|ActivateBlueKey))))
    (:NewEnumerator2
      (Utilities|FlowControl|DoOnce false
        (:Completed
          (CallFunction|ActivateGreenKey))))))

(fn ConstructionScript
  (bind _returnvalue (Rendering|Material|CreateDynamicMaterialInstance (Variables|Default|GetTotemBase) 1 "/Game/Materials/M_Glow.M_Glow" "None" :!class /Script/Engine.PrimitiveComponent))
  (bind _output_get (Variables|Default|SetTotemMaterial _returnvalue))
  (Rendering|Material|SetScalarParameterValue _output_get "Emission" (Variables|Default|GetEmissionIntensity) :!class /Script/Engine.MaterialInstanceDynamic)
  (Rendering|Material|SetVectorParameterValue _output_get "BaseColor" (Variables|Default|GetBaseColor) :!class /Script/Engine.MaterialInstanceDynamic))

(fn PlayTotemAnimationandSetEmission
  (Components|Timeline|PlayfromStart (Variables|Default|GetTotemRimTimeline))
  (Rendering|Material|SetScalarParameterValue (Variables|Default|GetTotemMaterial) "Emission" (Variables|Default|GetEmissionIntensityActive) :!class /Script/Engine.MaterialInstanceDynamic))

(fn SpawnKey
  (bind _returnvalue (Game|SpawnActorfromClass "/Game/Objects/Key/BP_KeyFixed.BP_KeyFixed_C" (Transformation|GetWorldTransform (Variables|Default|GetKeySpawnTransform)) "Undefined" 0 0))
  (return _returnvalue))

(fn ChangeActiveKeyColor
  (params (Frame1 :type Static%20Mesh%20Component%20Object%20Reference) (BaseColor :type Linear%20Color%20Structure) (Emission :type Float%20%28single-precision%29))
  (bind _returnvalue (Rendering|Material|CreateDynamicMaterialInstance Frame1 1 "/Game/Materials/M_Glow.M_Glow" "None" :!class /Script/Engine.PrimitiveComponent))
  (Rendering|Material|SetVectorParameterValue _returnvalue "BaseColor" BaseColor :!class /Script/Engine.MaterialInstanceDynamic)
  (Rendering|Material|SetScalarParameterValue _returnvalue "Emission" Emission :!class /Script/Engine.MaterialInstanceDynamic))

(fn GetTotemColor
  (params (Color :type EKeys%20Enum :default "NewEnumerator0"))
  (bind _totemscolor (Variables|Default|GetTotemsColor))
  (bind (_pink _blue _green) (Utilities|Struct|BreakColorsStruct _totemscolor))
  (switch Utilities|FlowControl|Switch|SwitchonEKeys Color
    (:NewEnumerator0
      (return _pink))
    (:NewEnumerator1
      (return _blue))
    (:NewEnumerator2
      (return _green))))