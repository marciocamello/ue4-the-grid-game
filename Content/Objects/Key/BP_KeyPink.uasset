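; BP_KeyPink is the pink key variant, a child Blueprint that sets up its own glowing look.
; Its construction script runs the parent's, then gives Frame1 and Frame2 each a dynamic M_Glow material instance on their second material slot.
; Both instances take their base color from GetKeyColor with a fixed key enum value and get a strong emission.
; The event graph holds only disabled stubs, adding no runtime logic.
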(event EventBeginPlay
  (|CallParentFunction) ; This node is disabled and will not be called.\nDrag off pins to build functionality.
)

(event Collision|EventActorBeginOverlap
  (params (OtherActor :type Actor%20Object%20Reference))
  (|CallParentFunction OtherActor) ; This node is disabled and will not be called.\nDrag off pins to build functionality.
)

(event EventTick
  (params (DeltaSeconds :type Float%20%28single-precision%29))
  (|CallParentFunction DeltaSeconds) ; This node is disabled and will not be called.\nDrag off pins to build functionality.
)

(fn ConstructionScript
  (bind _totemcolor (CallFunction|GetKeyColor "NewEnumerator0"))
  (|CallParentFunction)
  (bind _returnvalue (Rendering|Material|CreateDynamicMaterialInstance (Variables|Default|GetFrame1) 1 "/Game/Materials/M_Glow.M_Glow" "None" :!class /Script/Engine.PrimitiveComponent))
  (Rendering|Material|SetVectorParameterValue _returnvalue "BaseColor" _totemcolor :!class /Script/Engine.MaterialInstanceDynamic)
  (Rendering|Material|SetScalarParameterValue _returnvalue "Emission" 2e+01 :!class /Script/Engine.MaterialInstanceDynamic)
  (bind _returnvalue_2 (Rendering|Material|CreateDynamicMaterialInstance (Variables|Default|GetFrame2) 1 "/Game/Materials/M_Glow.M_Glow" "None" :!class /Script/Engine.PrimitiveComponent))
  (Rendering|Material|SetVectorParameterValue _returnvalue_2 "BaseColor" _totemcolor :!class /Script/Engine.MaterialInstanceDynamic)
  (Rendering|Material|SetScalarParameterValue _returnvalue_2 "Emission" 2e+01 :!class /Script/Engine.MaterialInstanceDynamic))