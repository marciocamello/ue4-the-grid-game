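; BP_Key is a colored key pickup that comes in pink, blue or green.
; Pickup returns the key's KeyColor, and GetKeyColor maps a key color to its matching entry in KeysColor.
; Two timelines are set up to spin Frame1 in yaw and Frame2 in pitch while bobbing the Core vertically, though no graph event starts them.
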(event EventBeginPlay)

(event Collision|EventActorBeginOverlap
  (params (OtherActor :type Actor%20Object%20Reference)))

(event EventTick
  (params (DeltaSeconds :type Float%20%28single-precision%29)))

(fn ConstructionScript)

(fn GetKeyColor
  (params (Color :type EKeys%20Enum :default "NewEnumerator0"))
  (bind _keyscolor (Variables|Default|GetKeysColor))
  (bind (_pink _blue _green) (Utilities|Struct|BreakColorsStruct _keyscolor))
  (switch Utilities|FlowControl|Switch|SwitchonEKeys Color
    (:NewEnumerator0
      (return _pink))
    (:NewEnumerator1
      (return _blue))
    (:NewEnumerator2
      (return _green))))

(fn Pickup
  (return (Variables|Default|GetKeyColor)))